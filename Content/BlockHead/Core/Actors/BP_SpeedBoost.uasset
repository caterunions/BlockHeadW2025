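; BP_SpeedBoost is a pickup actor that grants the player a temporary speed boost.
; It overrides the parent's OnPickup, runs the inherited logic, then passes its speed multiplier and duration to the player through ConsumeSpeedBoost.
; The event graph holds only disabled default events, so pickup detection and the effect itself are handled outside this Blueprint.
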(event EventBeginPlay
  (|CallParentFunction) ; This node is disabled and will not be called.\nDrag off pins to build functionality.
)

(event Collision|EventActorBeginOverlap
  (params (OtherActor :type Actor%20Object%20Reference))
  (|CallParentFunction OtherActor) ; This node is disabled and will not be called.\nDrag off pins to build functionality.
)

(event EventTick
  (params (DeltaSeconds :type Float%20%28single-precision%29))
  (|CallParentFunction DeltaSeconds) ; This node is disabled and will not be called.\nDrag off pins to build functionality.
)

(fn ConstructionScript
  (|CallParentFunction))

(fn OnPickup
  (|CallParentFunction)
  ;[0.03119 1 0.1322 0.5] Send powerup info to Player
  (Default|ConsumeSpeedBoost (Variables|Default|GetPlayer) (Variables|Default|GetSpeedMult) (Variables|Default|GetDuration)))